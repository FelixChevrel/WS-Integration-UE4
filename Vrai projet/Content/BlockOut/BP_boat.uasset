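; Blockout boat actor that rocks its Cube component to mimic bobbing on water.
; On BeginPlay it starts timeline X at a random play rate, so separate instances can move out of sync.
; Each update scales the timeline's vector output into relative roll and a gentler pitch, holding yaw at zero.
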(event EventBeginPlay
  (Components|Timeline|SetPlayRate (Variables|Default|GetX) (+ (* (Math|Random|RandomFloat) 2.0) 0.5))
  (bind (_direction _x _y) (Timeline|X Play)
    (:Update
      (Transformation|SetRelativeRotation (Variables|Default|GetCube) (Math|Rotator|MakeRotator (* _x 2e+01) (* _y 3.0) 0.0) false false))))

(fn ConstructionScript)