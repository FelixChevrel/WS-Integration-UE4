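; Spline-based Blueprint that builds a run of deformed meshes along a path, apparently a sidewalk judging by the asset name.
; The construction script divides the spline into sections sized by the actor's X scale and adds a Y-forward spline mesh for each.
; Tangents are clamped to section length, and each piece gets the MaterialTube material and query-and-physics collision.
; The event graph has no active logic.
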(event EventBeginPlay)

(event Collision|EventActorBeginOverlap
  (params (OtherActor :type Actor%20Object%20Reference)))

(event EventTick
  (params (DeltaSeconds :type Float%20%28single-precision%29)))

(fn ConstructionScript
  (bind _spline (Variables|Default|GetSpline))
  (Variables|Default|SetSectionsLength (* (.x (Transformation|GetActorScale3D)) 33.0))
  (for _index (range 0 (Math|Float|Truncate (/ (Spline|GetSplineLength (Variables|Default|GetSpline)) (Variables|Default|GetSectionsLength))))
    (bind _returnvalue (AddComponent|AddSplineMeshComponent false))
    (SplineMesh|SetForwardAxis _returnvalue "Y" true)
    (SplineMesh|SetStartandEnd _returnvalue (Spline|GetLocationatDistanceAlongSpline _spline (* _index (Variables|Default|GetSectionsLength)) "Local") (Math|Vector|ClampVectorSize (Spline|GetTangentatDistanceAlongSpline _spline (* _index (Variables|Default|GetSectionsLength)) "Local") 0.0 (Variables|Default|GetSectionsLength)) (Spline|GetLocationatDistanceAlongSpline _spline (* (+ _index 1) (Variables|Default|GetSectionsLength)) "Local") (Math|Vector|ClampVectorSize (Spline|GetTangentatDistanceAlongSpline _spline (* (+ _index 1) (Variables|Default|GetSectionsLength)) "Local") 0.0 (Variables|Default|GetSectionsLength)) true :!class /Script/Engine.SplineMeshComponent)
    (Rendering|Material|SetMaterial _returnvalue 0 (Variables|Default|GetMaterial_tube))
    (Collision|SetCollisionEnabled _returnvalue "QueryAndPhysics")
    (Variables|/Script/Engine.PrimitiveComponent|SetbTraceComplexOnMove _returnvalue true)))